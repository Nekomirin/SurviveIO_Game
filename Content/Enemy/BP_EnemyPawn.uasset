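; Enemy pawn that takes damage through a health component and explodes on death.
; Any damage is passed to HealthComponent, whose death event prints a debug message, unpossesses the controller, destroys the actor and spawns an explosion.
; Each tick sets the Body's absolute world rotation from speed times delta time, around an axis built from scalar speed, not movement direction.
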(event `self.ReceiveBeginPlay`
  (set `self.Health` 100.0))

(event `self.ReceiveTick`
  (params (DeltaSeconds :type "Float (single-precision)"))
  (bind _returnvalue (`KismetMathLibrary.VSize` (`self.GetVelocity` (`PawnMovementComponent.GetPawnOwner` (`self.FloatingPawnMovement`)))))
  (`SceneComponent.K2_SetWorldRotation` (`self.Body`) (`KismetMathLibrary.RotatorFromAxisAndAngle` (`KismetMathLibrary.Cross_VectorVector` (`KismetMathLibrary.Conv_DoubleToVector` _returnvalue) (`KismetMathLibrary.Vector_Down`)) (* DeltaSeconds _returnvalue)) false false))

(event `self.ReceiveAnyDamage`
  (params (Damage :type "Float (single-precision)") (DamageType :type "DamageType Object Reference") (InstigatedBy :type "Controller Object Reference") (DamageCauser :type "Actor Object Reference"))
  (`/Game/Health/HealthComponent.SetDamage` (`self.HealthComponent`) Damage))

(event `self.HealthComponent.ondeath`
  (`KismetSystemLibrary.PrintString` "Enemy Dead")
  (`Controller.UnPossess` (`self.GetController`))
  (`self.K2_DestroyActor`)
  (`GameplayStatics.SpawnEmitterAtLocation` "/Game/StarterContent/Particles/P_Explosion.P_Explosion" (`self.K2_GetActorLocation`)))

(fn `UserConstructionScript`)