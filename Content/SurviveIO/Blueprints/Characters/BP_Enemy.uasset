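; Zombie enemy character that attacks the main hero, takes damage through a health component and dies with sound and montage.
; Attack halts movement during the montage; the anim blueprint's OnHit event arms a hitbox that damages the hero once per swing.
; A world-space health bar widget binds to the health component and turns toward the player camera every tick.
; Death unpossesses the controller, hides the bar and disables capsule collision.
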(event `self.ReceiveAnyDamage`
  (params (Damage :type "Float (single-precision)") (DamageType :type "DamageType Object Reference") (InstigatedBy :type "Controller Object Reference") (DamageCauser :type "Actor Object Reference"))
  (`/Game/SurviveIO/Blueprints/Components/BPC_Health.SetDamage` (`self.BPC_Health`) Damage))

(event `self.ReceiveTick`
  (params (DeltaSeconds :type "Float (single-precision)"))
  (`SceneComponent.K2_SetWorldRotation` (`self.HealthbarWidget`) (`KismetMathLibrary.FindLookAtRotation` (`SceneComponent.K2_GetComponentLocation` (`self.HealthbarWidget`)) (`SceneComponent.K2_GetComponentLocation` (`PlayerCameraManager.TransformComponent` (`GameplayStatics.GetPlayerCameraManager` 0)))) false false))

(event `self.BPC_Health.OnDeath`
  (`self.Kill`))

(event `self.ReceiveBeginPlay`
  (bind _aswbp_health_bar (cast `/Game/SurviveIO/UI/WBP_HealthBar` (`WidgetComponent.GetUserWidgetObject` (`self.HealthbarWidget`))))
  (`/Game/SurviveIO/UI/WBP_HealthBar.InitHealthBar` _aswbp_health_bar (`self.BPC_Health`))
  (`self.InitOnHitEvent`))

(event `Attack`
  (`CharacterMovementComponent.DisableMovement` (`self.CharacterMovement`))
  (`|PlayMontage` (`self.Mesh`) "/Game/SurviveIO/Models/Zombari/Animations/AM_Attack.AM_Attack"
    (:`then`
      (`KismetSystemLibrary.Delay` 0.5)
      (`AudioComponent.Play` (`self.Growl`) 0.0))
    (:`OnCompleted`
      (`CharacterMovementComponent.SetMovementMode` (`self.CharacterMovement`) "MOVE_Walking" 0))))

(event `InitOnHitEvent`
  (bind _asabp_zombie (cast `/Game/SurviveIO/Models/Zombari/Animations/ABP_Zombie` (`SkeletalMeshComponent.GetAnimInstance` (`self.Mesh`))))
  (add `/Game/SurviveIO/Models/Zombari/Animations/ABP_Zombie.OnHit` _asabp_zombie (delegate `OnHit`)))

(event `OnHit`
  (set `PrimitiveComponent.bGenerateOverlapEvents` true (`self.Hitbox`)))

(event `self.Hitbox.OnComponentBeginOverlap`
  (params (OverlappedComponent :type "PrimitiveComponent Object Reference") (OtherActor :type "Actor Object Reference") (OtherComp :type "PrimitiveComponent Object Reference") (OtherBodyIndex :type Integer) (bFromSweep :type Boolean) (SweepResult :type "HitResult Structure (by ref)"))
  (bind _asbp_main_hero (cast `/Game/SurviveIO/Blueprints/Characters/BP_MainHero` OtherActor))
  (`GameplayStatics.ApplyDamage` _asbp_main_hero 20.0 (`self.GetController`) self)
  (set `PrimitiveComponent.bGenerateOverlapEvents` false (`self.Hitbox`))
  (`AudioComponent.Play` (`self.Punch`) 0.0))

(event `Kill`
  (bind _returnvalue (`self.GetController`))
  (`/Engine/EditorBlueprintResources/StandardMacros.IsValid` _returnvalue
    (:`Is Valid`
      (`GameplayStatics.PlaySoundAtLocation` "/Game/SurviveIO/Audio/SFX/Zombie/S_ZombieDeath_01.S_ZombieDeath_01" (`self.K2_GetActorLocation`) (struct) 1.0 1.0 0.0 null null null null)
      (`Controller.UnPossess` _returnvalue)
      (`SceneComponent.SetVisibility` (`self.HealthbarWidget`) false false)
      (`PrimitiveComponent.SetCollisionEnabled` (`self.CapsuleComponent`) "NoCollision")
      (`|PlayMontage` (`self.Mesh`) "/Game/SurviveIO/Models/Zombari/Animations/AM_Dying.AM_Dying"))))

(fn `UserConstructionScript`)